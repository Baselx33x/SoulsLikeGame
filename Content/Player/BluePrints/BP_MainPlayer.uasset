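; Main player Blueprint that handles the axe melee attack on left mouse click.
; When the weapon state is Equipped, a click randomly plays either a horizontal or a 360 high attack montage on the mesh.
; Player input is disabled for the duration of the swing and re-enabled only when the montage completes, with no handling for interruption.
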(event `Key|LeftMouseButton`
  (params (Key :type "Key Structure"))
  ;[0.08523 1 0.5416] Attack Animation
  (:`Pressed`
    (if (`|EnumEquality` (`self.m_PlayerWeaponState`) "PWS_Equipped")
      (switch `int` (`KismetMathLibrary.RandomIntegerInRange` 0 1)
        (:`0`
          (set `self.Montage to Play` "/Game/Player/Animations/Montages/Standing_Melee_Attack_Horizontal_With_Axe_Montage.Standing_Melee_Attack_Horizontal_With_Axe_Montage"))
        (:`1`
          (set `self.Montage to Play` "/Game/Player/Animations/Montages/Standing_Melee_Attack_360_High_With_Axe_Montage.Standing_Melee_Attack_360_High_With_Axe_Montage")))
      (`self.DisableInput` self (`GameplayStatics.GetPlayerController` 0))
      (`|PlayMontage` (`self.Mesh`) (`self.Montage to Play`)
        (:`OnCompleted`
          (`self.EnableInput` self (`GameplayStatics.GetPlayerController` 0)))))))

(event `self.ReceiveTick`
  (params (DeltaSeconds :type "Float (single-precision)")))

(fn `UserConstructionScript`)